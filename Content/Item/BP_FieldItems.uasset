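; BP_FieldItems is an item actor placed in the world whose appearance comes from its item class ID.
; On BeginPlay, a non-zero ItemClassID is converted to a row name and looked up in ItemClassTable.
; The row's static mesh is loaded asynchronously and applied to StaticMeshComponent.
; The Sphere collision radius is then resized to match the mesh's bounding sphere.
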(event `self.ReceiveBeginPlay`
  (bind _itemclassid (`self.ItemClassID`))
  (bind _staticmeshcomponent (`self.StaticMeshComponent`))
  (if (!= _itemclassid 0)
    (bind _returnvalue (`|GetDataTableRow` "/Game/Item/ItemClassTable.ItemClassTable" (`KismetStringLibrary.Conv_StringToName` (`KismetStringLibrary.Conv_IntToString` _itemclassid)))
      (:`then`
        (bind _object (`|LoadAsset` (`.StaticMesh_14_D4A01CB747D3CBE48A12A49BA5DECAE2` (break `/Game/Item/ItemClass` _returnvalue)))
          (:`Completed`
            (bind _asstatic_mesh (cast `StaticMesh` _object))
            (`StaticMeshComponent.SetStaticMesh` _staticmeshcomponent _asstatic_mesh)
            (`SphereComponent.SetSphereRadius` (`self.Sphere`) (`.SphereRadius` (`KismetSystemLibrary.GetComponentBounds` _staticmeshcomponent)) true)))))))

(fn `UserConstructionScript`)